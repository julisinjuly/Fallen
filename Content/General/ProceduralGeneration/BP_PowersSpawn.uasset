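; BP_PowersSpawn is a spawner actor that periodically creates BP_Powers actors at its Billboard component's location.
; On BeginPlay it attaches itself to the BP_Checkpoint found in the level, keeping its world transform.
; Tick feeds a randomized Delay of roughly ten seconds, which acts as a repeating spawn timer.
; A random Select chooses the class to spawn, though every listed option is BP_Powers.
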(event EventBeginPlay
  (bind _returnvalue (Actor|GetActorOfClass "/Game/General/ChechPoints/BP_Checkpoint.BP_Checkpoint_C"))
  (Utilities|IsValid _returnvalue
    (:Is%20Valid
      (Transformation|AttachActorToActor self _returnvalue "None" "KeepWorld" "KeepWorld" "KeepWorld" true))))

(event EventTick
  (params (DeltaSeconds :type Float%20%28single-precision%29))
  (Utilities|FlowControl|Delay (Math|Random|RandomFloatinRange 1e+01 11.0))
  (Game|SpawnActorfromClass (Utilities|Select :Index (Math|Random|RandomIntegerinRange 0 6) :Option%200 "/Game/General/Enemies/Powers_Enemies/BP_Powers.BP_Powers_C" :Option%201 "/Game/General/Enemies/Powers_Enemies/BP_Powers.BP_Powers_C" :Option%202 "/Game/General/Enemies/Powers_Enemies/BP_Powers.BP_Powers_C" :Option%203 "/Game/General/Enemies/Powers_Enemies/BP_Powers.BP_Powers_C") (Math|Transform|MakeTransform (Transformation|GetWorldLocation (Variables|Default|GetBillboard)) "0, 0, 0" "1.000000,1.000000,1.000000") "Undefined" "MultiplyWithRoot" 0 0))

(fn ConstructionScript)