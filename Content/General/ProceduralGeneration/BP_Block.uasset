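; Procedural block actor that builds a NumX by NumY grid of randomly picked streamed level instances around itself on BeginPlay.
; SpecificLevelIno entries override the default level pool at fixed or randomized cells, and each instance gets a random quarter-turn yaw.
; After spawning, the actor jumps to the first PlayerStart if a player character exists.
; Tick sinks only the actor, destroying it at BP_IslandDestrcuctLocation's height; construction-script cube generation is disconnected.
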(event EventBeginPlay
  (CallFunction|CheckforEntriesThatNeedCoordinates)
  (for _index (range 0 (- (Variables|Nums|GetNumX) 1))
    (Variables|Loops|SetLoopX _index)
    (for _index_2 (range 0 (- (Variables|Nums|GetNumY) 1))
      (Variables|Loops|SetLoopY _index_2)
      (bind (_leveldetails1 _bfoundinformation_1) (CallFunction|CheckforSpecificLevelInfo))
      (if _bfoundinformation_1
        (CallFunction|PickandSpawnLeveltoArray (.LevelNames (Utilities|Struct|BreakF_SpecificLevelInfo _leveldetails1)))
        (else
          (CallFunction|PickandSpawnLeveltoArray (Variables|Default|GetLevelNames))))))
  (bind _outactors (Actor|GetAllActorsOfClass "/Script/Engine.PlayerStart"))
  (Utilities|IsValid (Utilities|Array|Get(acopy) _outactors)
    (:Is%20Valid
      (Utilities|IsValid (Game|GetPlayerCharacter 0)
        (:Is%20Valid
          (Transformation|SetActorLocation (Transformation|GetActorLocation (Utilities|Array|Get(acopy) _outactors)) false false))))))

(event EventTick
  (params (DeltaSeconds :type Float%20%28single-precision%29))
  ;[0.03021 0.03021 0.03021] Moving Islands
  (Transformation|AddActorWorldOffset self "0.000000,0.000000,-5.000000")
  (bind _returnvalue (Actor|GetActorOfClass "/Game/General/CustomBP/TargetPoints/BP_IslandDestrcuctLocation.BP_IslandDestrcuctLocation_C"))
  (if (<= (.z (Transformation|GetActorLocation self)) (.z (Transformation|GetActorLocation _returnvalue)))
    (Actor|DestroyActor)))

(fn ConstructionScript)

(fn CenterLoopX
  (return (+ (- (* (Variables|Loops|GetLoopX) (Variables|Default|GetLevelSize)) (/ (* (Variables|Nums|GetNumX) (Variables|Default|GetLevelSize)) 2.0)) (/ (Variables|Default|GetLevelSize) 2.0))))

(fn CenterLoopY
  (return (+ (- (* (Variables|Loops|GetLoopY) (Variables|Default|GetLevelSize)) (/ (* (Variables|Nums|GetNumY) (Variables|Default|GetLevelSize)) 2.0)) (/ (Variables|Default|GetLevelSize) 2.0))))

(fn PickandSpawnLeveltoArray
  (params (LevelNames :type Array%20of%20Names))
  (bind _returnvalue (Class|LevelStreaming|CreateInstance (Class|GameplayStatics|GetStreamingLevel (Utilities|Array|Get(acopy) LevelNames (Math|Random|RandomIntegerinRange 0 (Utilities|Array|LastIndex LevelNames)))) (Utilities|String|Append (Utilities|String|ToString(Integer) (Variables|Loops|GetLoopX)) "x" (Utilities|String|ToString(Integer) (Variables|Loops|GetLoopY)) (Utilities|GetDisplayName self))))
  (Utilities|IsValid _returnvalue
    (:Is%20Valid
      (Variables|/Script/Engine.LevelStreaming|SetLevelTransform _returnvalue (Math|Transform|MakeTransform (+ (Math|Vector|MakeVector (CallFunction|CenterLoopX) (CallFunction|CenterLoopY) 0.0) (Transformation|GetActorLocation)) (Math|Rotator|MakeRotator 0.0 0.0 (* (Math|Random|RandomIntegerinRange 0 3) 9e+01))))
      (Variables|/Script/Engine.LevelStreaming|SetbShouldBeLoaded _returnvalue true)
      (Variables|/Script/Engine.LevelStreaming|SetbShouldBeLoaded _returnvalue true)
      (Variables|/Script/Engine.LevelStreaming|SetbShouldBeVisible _returnvalue true))))

(fn CheckforSpecificLevelInfo
  (LocalVariables|SetbFoundInformation? false)
  (for _array_element (Variables|Default|GetSpecificLevelIno)
    (if (not (LocalVariables|GetbFoundInformation?))
      (if (and (== (- (Math|Float|Round (.X (Math|Vector|BreakVector (.Coordinates (Utilities|Struct|BreakF_SpecificLevelInfo _array_element))))) 1) (Variables|Loops|GetLoopX)) (== (- (Math|Float|Round (.Y (Math|Vector|BreakVector (.Coordinates (Utilities|Struct|BreakF_SpecificLevelInfo _array_element))))) 1) (Variables|Loops|GetLoopY)))
        (LocalVariables|SetLevelDetails _array_element)
        (LocalVariables|SetbFoundInformation? true))))
  (return (LocalVariables|GetLevelDetails) (LocalVariables|GetbFoundInformation?)))

(fn CheckforEntriesThatNeedCoordinates
  (for (_array_element _array_index) (Variables|Default|GetSpecificLevelIno)
    (if (.bGetRandomCoordinatesOnBeginPlay (Utilities|Struct|BreakF_SpecificLevelInfo _array_element))
      (Utilities|Array|SetArrayElem (Variables|Default|GetSpecificLevelIno) _array_index (Utilities|Struct|MakeF_SpecificLevelInfo (Math|Vector|MakeVector (Math|Conversions|ToFloat(Integer) (Math|Random|RandomIntegerinRange 0 (Variables|Nums|GetNumX))) (Math|Conversions|ToFloat(Integer) (Math|Random|RandomIntegerinRange 0 (Variables|Nums|GetNumY))) 0.0) (.LevelNames (Utilities|Struct|BreakF_SpecificLevelInfo _array_element)) (.bGetRandomCoordinatesOnBeginPlay (Utilities|Struct|BreakF_SpecificLevelInfo _array_element))))))
  (return))