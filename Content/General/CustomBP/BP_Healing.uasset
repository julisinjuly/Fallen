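; BP_Healing is a health pickup that adds a fixed amount to the first-person character's CurrentHealth on overlap, then destroys itself.
; The overlap handler casts to BP_FirstPersonCharacter and applies no maximum-health clamp.
; BeginPlay finds BP_Keeper and loops over all BP_Healing actors with an empty body, as the node attaching them to the Keeper's Box is disconnected.
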(event EventBeginPlay
  (bind _returnvalue (Actor|GetActorOfClass "/Game/General/ProceduralGeneration/BP_Keeper.BP_Keeper_C"))
  (bind _outactors (Actor|GetAllActorsOfClass "BP_Healing_C"))
  (for _array_element _outactors
    _))

(event Collision|EventActorBeginOverlap
  (params (OtherActor :type Actor%20Object%20Reference))
  (bind _asbp_first_person_character (Utilities|Casting|CastToBP_FirstPersonCharacter OtherActor))
  (bind _output_get (Variables|Default|SetBP%20First%20Person%20Character%20Ref _asbp_first_person_character))
  (Variables|/Game/FirstPerson/Blueprints/BP_FirstPersonCharacter.BP_FirstPersonCharacter_C|SetCurrentHealth (Variables|Default|GetBP%20First%20Person%20Character%20Ref) (+ (Variables|/Game/FirstPerson/Blueprints/BP_FirstPersonCharacter.BP_FirstPersonCharacter_C|GetCurrentHealth _output_get) 25.0))
  (Actor|DestroyActor))

(fn ConstructionScript)