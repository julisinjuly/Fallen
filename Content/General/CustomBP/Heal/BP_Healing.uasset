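; BP_Healing is a healing pickup that adds a fixed amount to the player's CurrentHealth on overlap.
; It casts the overlapping actor to BP_FirstPersonCharacter and increases its health directly, without a clamp.
; It then plays a healing sound, hides its mesh, spawns an attached effect and destroys itself after a short delay.
; Overlap stays active during that delay, so re-entering can heal again.
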(event Collision|EventActorBeginOverlap
  (params (OtherActor :type Actor%20Object%20Reference))
  (bind _asbp_first_person_character (Utilities|Casting|CastToBP_FirstPersonCharacter OtherActor))
  (bind _output_get (Variables|Default|SetBP%20First%20Person%20Character%20Ref _asbp_first_person_character))
  (Variables|/Game/FirstPerson/Blueprints/BP_FirstPersonCharacter.BP_FirstPersonCharacter_C|SetCurrentHealth (Variables|Default|GetBP%20First%20Person%20Character%20Ref) (+ (Variables|/Game/FirstPerson/Blueprints/BP_FirstPersonCharacter.BP_FirstPersonCharacter_C|GetCurrentHealth _output_get) 5e+01))
  (Audio|PlaySoundatLocation "/Game/General/SoundDesign/SoundMontages/Cue_Healing.Cue_Healing" (- (Transformation|GetActorLocation self) "0.000000,0.000000,60.000000") "0, 0, 0" 1.0 1.0 0.0 0 0 0 0)
  (Rendering|SetVisibility (Variables|Default|GetStaticMesh) false false)
  (Rendering|SetVisibility (Variables|Default|GetStaticMesh) false false)
  (Niagara|SpawnSystemAttached "/Game/General/VFX/VFX_BP/NS_BowlOfTheUniverse3.NS_BowlOfTheUniverse3" (Variables|Default|GetStaticMesh) "None" "0, 0, 0" "0, 0, 0" "KeepRelativeOffset" false)
  (Utilities|FlowControl|Delay 3.0)
  (Actor|DestroyActor))

(fn ConstructionScript)