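; BP_Powers is an AI enemy that weakens and damages the player on contact and dies when its health runs out.
; BeginPlay passes a behavior tree and player sensing target to AI_PowersController, while a delayed Tick sphere-traces for damage when the player is near.
; Overlap deals damage and slows player movement; leaving restores speed and sets Angel and projectile damage.
; Incoming hits update a health widget, then trigger particles and destruction at zero.
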(event Custom|Damage%20the%20MC
  ;[0.03021 0.03021 0.03021] Damage system
  (if (Variables|Default|GetbIsOverlappingCharacter?)
    (Utilities|Time|SetTimerbyFunctionName 0 "Damage the MC" 1.0 true)
    (Game|Damage|ApplyDamage (Variables|Default|GetCharacterRef) 5.0 0 0)))

(event EventBeginPlay
  ;[0.03854 0.03854 0.03854] Setting up AI controller
  (bind _asai_powers_controller (Utilities|Casting|CastToAI_PowersController (AI|GetAIController self)))
  (Default|SetUpAIC _asai_powers_controller (Variables|Default|GetBT) (Game|Player|GetPlayerPawn 0)))

(event Collision|EventActorBeginOverlap
  (params (OtherActor :type Actor%20Object%20Reference))
  ;[0.03021 0.03021 0.03021] Damage system
  (bind _asbp_first_person_character (Utilities|Casting|CastToBP_FirstPersonCharacter OtherActor))
  (Variables|Default|SetCharacterRef _asbp_first_person_character)
  (Variables|Default|SetbIsOverlappingCharacter? true)
  (CallFunction|DamagetheMC)
  (Variables|/Script/Engine.CharacterMovementComponent|SetMaxFlySpeed (Variables|/Script/Engine.Character|GetCharacterMovement (Game|GetPlayerCharacter 0)) 359.0)
  (Variables|/Script/Engine.CharacterMovementComponent|SetMaxWalkSpeed (Variables|/Script/Engine.Character|GetCharacterMovement (Game|GetPlayerCharacter 0)) 5e+02)
  (Variables|/Script/Engine.CharacterMovementComponent|SetMaxCustomMovementSpeed (Variables|/Script/Engine.Character|GetCharacterMovement (Game|GetPlayerCharacter 0)) 3e+02)
  (Variables|/Script/Engine.CharacterMovementComponent|SetMaxAcceleration (Variables|/Script/Engine.Character|GetCharacterMovement (Game|GetPlayerCharacter 0)) 5e+02)
  (Development|PrintString "weakened"))

(event Collision|EventActorEndOverlap
  (params (OtherActor :type Actor%20Object%20Reference))
  (bind _returnvalue (Game|GetPlayerCharacter 0))
  (bind _returnvalue_2 (Game|GetPlayerCharacter 0))
  (bind _charactermovement (Variables|/Script/Engine.Character|GetCharacterMovement _returnvalue))
  (bind _charactermovement_2 (Variables|/Script/Engine.Character|GetCharacterMovement _returnvalue_2))
  ;[0.03021 0.03021 0.03021] Damage system
  (Utilities|Casting|CastToBP_FirstPersonCharacter OtherActor)
  (Variables|Default|SetbIsOverlappingCharacter? false)
  (Utilities|IsValid _charactermovement
    (:Is%20Valid
      (Variables|/Script/Engine.CharacterMovementComponent|SetMaxFlySpeed _charactermovement 5e+03)
      (Utilities|IsValid _charactermovement_2
        (:Is%20Valid
          (Variables|/Script/Engine.CharacterMovementComponent|SetMaxWalkSpeed _charactermovement_2 1e+03)
          (Variables|/Script/Engine.CharacterMovementComponent|SetMaxCustomMovementSpeed (Variables|/Script/Engine.Character|GetCharacterMovement (Game|GetPlayerCharacter 0)) 1e+03)
          (Variables|/Script/Engine.CharacterMovementComponent|SetMaxAcceleration (Variables|/Script/Engine.Character|GetCharacterMovement (Game|GetPlayerCharacter 0)) 2.15e+03)
          (bind _outactors (Actor|GetAllActorsOfClass "/Game/General/Enemies/Angel_Enemy/Angel/BP_Angel.BP_Angel_C"))
          (for _array_element _outactors
            (bind _asbp_angel (Utilities|Casting|CastToBP_Angel _array_element))
            (Variables|/Game/General/Enemies/Angel_Enemy/Angel/BP_Angel.BP_Angel_C|SetDamage _asbp_angel 5.0)
            (bind _outactors_2 (Actor|GetAllActorsOfClass "/Game/FirstPerson/Blueprints/BP_FirstPersonProjectile.BP_FirstPersonProjectile_C"))
            (for _array_element_2 _outactors_2
              (bind _asbp_first_person_projectile (Utilities|Casting|CastToBP_FirstPersonProjectile _array_element_2))
              (Variables|/Game/FirstPerson/Blueprints/BP_FirstPersonProjectile.BP_FirstPersonProjectile_C|SetBulletDamage _asbp_first_person_projectile 2e+01))))))))

(event Game|Damage|EventAnyDamage
  (params (Damage :type Float%20%28single-precision%29) (DamageType :type Damage%20Type%20Object%20Reference) (InstigatedBy :type Controller%20Object%20Reference) (DamageCauser :type Actor%20Object%20Reference))
  (Audio|PlaySoundatLocation "/Game/General/SoundDesign/SoundMontages/Cue_EnemyHit.Cue_EnemyHit" (Transformation|GetActorLocation self) "0, 0, 0" 1.0 1.0 0.0 0 0 0 0)
  (bind _output_get (Variables|Health|SetCurrentHealth (- (Variables|Health|GetCurrentHealth) (* Damage 1e+02))))
  (bind _aswbp_enemy_health (Utilities|Casting|CastToWBP_EnemyHealth (UserInterface|GetUserWidgetObject (Variables|Default|GetWidget))))
  (bind _output_get_2 (Variables|Default|SetWBPEnemyHealth _aswbp_enemy_health))
  (Default|UpdateHealth _output_get_2 (Math|Integer|Clamp(Integer) _output_get 0 (Variables|Health|GetMaxHealth)))
  (if (<= (Variables|Health|GetCurrentHealth) 0)
    (Effects|SpawnEmitterAttached "/Engine/Tutorial/SubEditors/TutorialAssets/TutorialParticleSystem.TutorialParticleSystem" (Variables|Collision|GetCapsuleComponent) "None")
    (Utilities|FlowControl|Delay 2.0)
    (Actor|DestroyActor)))

(event EventTick
  (params (DeltaSeconds :type Float%20%28single-precision%29))
  (bind _self self)
  (bind _returnvalue (Transformation|GetActorLocation _self))
  ;[0.05521 0.05521 0.05521] Launch  Impulse
  (Utilities|FlowControl|Delay 5.0)
  (if (< (Transformation|GetDistanceTo self (Game|GetPlayerCharacter 0)) 2e+02)
    (bind _outactors (Actor|GetAllActorsOfClass "/Game/General/Enemies/Angel_Enemy/Angel/BP_Angel.BP_Angel_C"))
    (bind _outhit (Collision|SphereTraceByChannel _returnvalue (+ _returnvalue (* (Physics|GetCenterOfMass (Variables|Collision|GetCapsuleComponent _self) "None") 3.5e+02)) 7e+02 "TraceTypeQuery1" false _outactors "ForDuration"))
    (Game|Damage|ApplyDamage (.HitActor (Collision|BreakHitResult _outhit)) 5.0 0 0)))

(fn ConstructionScript)