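; BP_Turret is an enemy turret that hands its behavior tree and the player pawn to AI_TurretController on BeginPlay.
; When PawnSensing sees the player character or TurretShoots is called, it waits on a shared three-second Delay.
; It then spawns two scaled-up BP_CustomPrijectile actors at its Cone and Cube components, rotated toward the player.
; Overlapping the player character calls ApplyDamage on it, with no damage amount set.
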(event OnSeePawn(PawnSensing)
  (params (Pawn :type Pawn%20Object%20Reference))
  ;[1 1 1] Shooting logic
  (Utilities|Casting|CastToBP_FirstPersonCharacter Pawn)
  (Utilities|FlowControl|Delay 3.0)
  (Game|SpawnActorfromClass "/Game/General/Enemies/BP_CustomPrijectile.BP_CustomPrijectile_C" (Math|Transform|MakeTransform (Transformation|GetWorldLocation (Variables|Default|GetCone)) (Math|Rotator|FindLookatRotation (Transformation|GetActorLocation) (Transformation|GetActorLocation (Game|Player|GetPlayerPawn 0))) "5.000000,5.000000,5.000000") "AlwaysSpawn" "MultiplyWithRoot" 0 0)
  (Game|SpawnActorfromClass "/Game/General/Enemies/BP_CustomPrijectile.BP_CustomPrijectile_C" (Math|Transform|MakeTransform (Transformation|GetWorldLocation (Variables|Default|GetCube)) (Math|Rotator|FindLookatRotation (Transformation|GetActorLocation) (Transformation|GetActorLocation (Game|Player|GetPlayerPawn 0))) "5.000000,5.000000,5.000000") "AlwaysSpawn" "MultiplyWithRoot" 0 0))

(event Custom|TurretShoots
  ;[1 1 1] Shooting logic
  (Utilities|FlowControl|Delay 3.0)
  (Game|SpawnActorfromClass "/Game/General/Enemies/BP_CustomPrijectile.BP_CustomPrijectile_C" (Math|Transform|MakeTransform (Transformation|GetWorldLocation (Variables|Default|GetCone)) (Math|Rotator|FindLookatRotation (Transformation|GetActorLocation) (Transformation|GetActorLocation (Game|Player|GetPlayerPawn 0))) "5.000000,5.000000,5.000000") "AlwaysSpawn" "MultiplyWithRoot" 0 0)
  (Game|SpawnActorfromClass "/Game/General/Enemies/BP_CustomPrijectile.BP_CustomPrijectile_C" (Math|Transform|MakeTransform (Transformation|GetWorldLocation (Variables|Default|GetCube)) (Math|Rotator|FindLookatRotation (Transformation|GetActorLocation) (Transformation|GetActorLocation (Game|Player|GetPlayerPawn 0))) "5.000000,5.000000,5.000000") "AlwaysSpawn" "MultiplyWithRoot" 0 0))

(event EventBeginPlay
  ;[1 1 1] Setting up custom controller
  (bind _asai_turret_controller (Utilities|Casting|CastToAI_TurretController (AI|GetAIController self)))
  (Default|SetUpAIC _asai_turret_controller (Variables|Default|GetBT) (Game|Player|GetPlayerPawn 0)))

(event Collision|EventActorBeginOverlap
  (params (OtherActor :type Actor%20Object%20Reference))
  ;[1 1 1] Apllying Damage on overlap
  (bind _asbp_first_person_character (Utilities|Casting|CastToBP_FirstPersonCharacter OtherActor))
  (Game|Damage|ApplyDamage _asbp_first_person_character 0.0 0 0))

(fn ConstructionScript)