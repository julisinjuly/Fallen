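; Rotating four-sided shield for the Principalities enemy, intended to reflect the main character's missiles.
; Tick continuously yaws ShieldRotator by a fixed step, without delta-time scaling.
; A hit on the front, back, left or right shield fires a debug-drawn Visibility line trace along that component's forward vector and applies fixed damage to the traced actor.
; The reflection is trace-based damage; no projectile is redirected or spawned.
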(event OnComponentHit(ShiledRight)
  (params (HitComponent :type Primitive%20Component%20Object%20Reference) (OtherActor :type Actor%20Object%20Reference) (OtherComp :type Primitive%20Component%20Object%20Reference) (NormalImpulse :type Vector :default "0, 0, 0") (Hit :type Hit%20Result%20Structure%20%28by%20ref%29))
  (bind _returnvalue (Transformation|GetWorldLocation HitComponent))
  ;[0.02187 0.02187 0.02187] Reflecting MC mislies
  (bind _outhit (Collision|LineTraceByChannel _returnvalue (+ _returnvalue (* (Math|Vector|GetForwardVector HitComponent) 8e+02)) "TraceTypeQuery1" false 0 "ForDuration"))
  (Game|Damage|ApplyDamage (.HitActor (Collision|BreakHitResult _outhit)) 2e+01 0 0))

(event OnComponentHit(ShieldLeft)
  (params (HitComponent :type Primitive%20Component%20Object%20Reference) (OtherActor :type Actor%20Object%20Reference) (OtherComp :type Primitive%20Component%20Object%20Reference) (NormalImpulse :type Vector :default "0, 0, 0") (Hit :type Hit%20Result%20Structure%20%28by%20ref%29))
  (bind _returnvalue (Transformation|GetWorldLocation HitComponent))
  ;[0.02187 0.02187 0.02187] Reflecting MC mislies
  (bind _outhit (Collision|LineTraceByChannel _returnvalue (+ _returnvalue (* (Math|Vector|GetForwardVector HitComponent) 8e+02)) "TraceTypeQuery1" false 0 "ForDuration"))
  (Game|Damage|ApplyDamage (.HitActor (Collision|BreakHitResult _outhit)) 2e+01 0 0))

(event OnComponentHit(ShieldFront)
  (params (HitComponent :type Primitive%20Component%20Object%20Reference) (OtherActor :type Actor%20Object%20Reference) (OtherComp :type Primitive%20Component%20Object%20Reference) (NormalImpulse :type Vector :default "0, 0, 0") (Hit :type Hit%20Result%20Structure%20%28by%20ref%29))
  (bind _returnvalue (Transformation|GetWorldLocation HitComponent))
  ;[0.02187 0.02187 0.02187] Reflecting MC mislies
  (bind _outhit (Collision|LineTraceByChannel _returnvalue (+ _returnvalue (* (Math|Vector|GetForwardVector HitComponent) 8e+02)) "TraceTypeQuery1" false 0 "ForDuration"))
  (Game|Damage|ApplyDamage (.HitActor (Collision|BreakHitResult _outhit)) 2e+01 0 0))

(event OnComponentHit(ShildBack)
  (params (HitComponent :type Primitive%20Component%20Object%20Reference) (OtherActor :type Actor%20Object%20Reference) (OtherComp :type Primitive%20Component%20Object%20Reference) (NormalImpulse :type Vector :default "0, 0, 0") (Hit :type Hit%20Result%20Structure%20%28by%20ref%29))
  (bind _returnvalue (Transformation|GetWorldLocation HitComponent))
  ;[0.02187 0.02187 0.02187] Reflecting MC mislies
  (bind _outhit (Collision|LineTraceByChannel _returnvalue (+ _returnvalue (* (Math|Vector|GetForwardVector HitComponent) 8e+02)) "TraceTypeQuery1" false 0 "ForDuration"))
  (Game|Damage|ApplyDamage (.HitActor (Collision|BreakHitResult _outhit)) 2e+01 0 0))

(event EventTick
  (params (DeltaSeconds :type Float%20%28single-precision%29))
  (Transformation|AddWorldRotation (Variables|Default|GetShieldRotator) "0.000000,5.000000,0.000000" false false))

(event EventBeginPlay)

(fn ConstructionScript)