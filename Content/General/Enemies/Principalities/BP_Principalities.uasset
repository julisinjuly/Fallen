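; Principalities enemy whose AI controller receives a behavior tree and the player pawn, with a constantly rotating shield.
; Shield hits trace a debug reflection ray and damage the player directly; a shooting event spawns a delayed projectile from the shield.
; Player overlap applies damage and sets a looping damage timer.
; Incoming damage is scaled up, updates a health widget, and triggers particles and delayed destruction at zero health.
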(event OnComponentHit(ShieldCollision)
  (params (HitComponent :type Primitive%20Component%20Object%20Reference) (OtherActor :type Actor%20Object%20Reference) (OtherComp :type Primitive%20Component%20Object%20Reference) (NormalImpulse :type Vector :default "0, 0, 0") (Hit :type Hit%20Result%20Structure%20%28by%20ref%29))
  ;[0.04271 0.04271 0.04271] Reflecting the missile
  (CallFunction|ReflectionMisille))

(event OnComponentHit(ShieldCollision1)
  (params (HitComponent :type Primitive%20Component%20Object%20Reference) (OtherActor :type Actor%20Object%20Reference) (OtherComp :type Primitive%20Component%20Object%20Reference) (NormalImpulse :type Vector :default "0, 0, 0") (Hit :type Hit%20Result%20Structure%20%28by%20ref%29))
  ;[0.04271 0.04271 0.04271] Reflecting the missile
  (CallFunction|ReflectionMisille Hit))

(event OnComponentHit(ShieldCollision2)
  (params (HitComponent :type Primitive%20Component%20Object%20Reference) (OtherActor :type Actor%20Object%20Reference) (OtherComp :type Primitive%20Component%20Object%20Reference) (NormalImpulse :type Vector :default "0, 0, 0") (Hit :type Hit%20Result%20Structure%20%28by%20ref%29))
  ;[0.04271 0.04271 0.04271] Reflecting the missile
  (CallFunction|ReflectionMisille Hit))

(event OnComponentHit(ShieldCollision3)
  (params (HitComponent :type Primitive%20Component%20Object%20Reference) (OtherActor :type Actor%20Object%20Reference) (OtherComp :type Primitive%20Component%20Object%20Reference) (NormalImpulse :type Vector :default "0, 0, 0") (Hit :type Hit%20Result%20Structure%20%28by%20ref%29))
  ;[0.04271 0.04271 0.04271] Reflecting the missile
  (CallFunction|ReflectionMisille Hit))

(event Custom|Damage%20the%20MC
  ;[0.03021 0.03021 0.03021] Damage system
  (if (Variables|Default|GetbIsOverlappingCharacter?)
    (Utilities|Time|SetTimerbyFunctionName 0 "Damage the MC" 1.0 true)
    (Game|Damage|ApplyDamage (Variables|Default|GetCharacterRef) 3.0 0 0)))

(event Custom|ShootAtTheMC
  (bind _principalitiesshield (Variables|Default|GetPrincipalitiesShield))
  ;[0.05104 0.05104 0.05104] Shooting
  (Utilities|FlowControl|Delay 0.8)
  (Game|SpawnActorfromClass "/Game/FirstPerson/Blueprints/BP_FirstPersonProjectile.BP_FirstPersonProjectile_C" (Math|Transform|MakeTransform (Transformation|GetWorldLocation _principalitiesshield) (Transformation|GetWorldRotation _principalitiesshield)) "AlwaysSpawn" "MultiplyWithRoot" 0 0))

(event EventBeginPlay
  ;[0.03854 0.03854 0.03854] Setting up AI controller
  (Utilities|FlowControl|Sequence
    (:then_0
      (bind _asai_principalities_controller (Utilities|Casting|CastToAI_PrincipalitiesController (AI|GetAIController self)))
      (Default|SetUpAIC _asai_principalities_controller (Variables|Default|GetBT) (Game|Player|GetPlayerPawn 0)))))

(event Collision|EventActorBeginOverlap
  (params (OtherActor :type Actor%20Object%20Reference))
  ;[0.03021 0.03021 0.03021] Damage system
  (bind _asbp_first_person_character (Utilities|Casting|CastToBP_FirstPersonCharacter OtherActor))
  (Variables|Default|SetCharacterRef _asbp_first_person_character)
  (Variables|Default|SetbIsOverlappingCharacter? true)
  (CallFunction|DamagetheMC))

(event Collision|EventActorEndOverlap
  (params (OtherActor :type Actor%20Object%20Reference))
  ;[0.03021 0.03021 0.03021] Damage system
  (Utilities|Casting|CastToBP_FirstPersonCharacter OtherActor)
  (Variables|Default|SetbIsOverlappingCharacter? false))

(event Game|Damage|EventAnyDamage
  (params (Damage :type Float%20%28single-precision%29) (DamageType :type Damage%20Type%20Object%20Reference) (InstigatedBy :type Controller%20Object%20Reference) (DamageCauser :type Actor%20Object%20Reference))
  ;[0.05104 0.05104 0.05104] Receiving damage system
  (bind _output_get (Variables|Health|SetCurrentHealth (- (Variables|Health|GetCurrentHealth) (* Damage 1e+02))))
  (bind _aswbp_enemy_health (Utilities|Casting|CastToWBP_EnemyHealth (UserInterface|GetUserWidgetObject (Variables|Default|GetWidget))))
  (bind _output_get_2 (Variables|Default|SetWBPEnemyHealth _aswbp_enemy_health))
  (Default|UpdateHealth _output_get_2 (Math|Integer|Clamp(Integer) _output_get 0 (Variables|Health|GetMaxHealth)))
  (if (<= (Variables|Health|GetCurrentHealth) 0)
    (Effects|SpawnEmitterAttached "/Engine/Tutorial/SubEditors/TutorialAssets/TutorialParticleSystem.TutorialParticleSystem" (Variables|Collision|GetCapsuleComponent) "None")
    (Utilities|FlowControl|Delay 2.0)
    (Actor|DestroyActor)))

(event EventTick
  (params (DeltaSeconds :type Float%20%28single-precision%29))
  ;[0.03438 0.03438 0.03438] Rotating the shield
  (Transformation|AddRelativeRotation (Variables|Default|GetShieldRotator) "0.000000,5.000000,0.000000" false false))

(fn ConstructionScript)

(fn ShootingattheMC1
  (Game|SpawnActorfromClass "/Game/FirstPerson/Blueprints/BP_FirstPersonProjectile.BP_FirstPersonProjectile_C" (Math|Transform|MakeTransform (Transformation|GetSocketLocation (Variables|Default|GetPrincipalitiesShield) "None") "0, 0, 0" "1.000000,1.000000,1.000000") "Undefined" "MultiplyWithRoot" 0 0))

(fn ReflectionMisille
  (params (ShiledHitResult :type Hit%20Result%20Structure))
  (bind (_bblockinghit _binitialoverlap _time _distance _location _impactpoint _normal _impactnormal _physmat _hitactor _hitcomponent _hitbonename _bonename _hititem _elementindex _faceindex _tracestart _traceend) (Collision|BreakHitResult ShiledHitResult))
  (Collision|LineTraceByChannel _location (+ _location (* (Math|Vector|GetReflectionVector (Math|Vector|GetUnitDirection(Vector) _tracestart _traceend) _normal) 7e+03)) "TraceTypeQuery1" false 0 "ForOneFrame")
  (Game|Damage|ApplyDamage (Game|Player|GetPlayerPawn 0) 0.5 0 0)
  (Development|PrintString "ShieldIsHit!"))