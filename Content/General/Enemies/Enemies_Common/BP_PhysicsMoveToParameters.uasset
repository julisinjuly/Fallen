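; Actor component for enemy characters that prepares the owner for physics-driven movement, judging by its name and setup.
; Setup caches the owning Character and its capsule, enables physics simulation on the capsule, turns gravity off and applies the component's linear and angular damping.
; It only warns if the owner is not a Character; Tick is empty and a capsule rotation reset is left unconnected.
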(event Custom|Setup
  (bind _ascharacter (Utilities|Casting|CastToCharacter (Components|GetOwner))
    (:then
      (bind _output_get (Variables|Default|SetOwningCharacterRef _ascharacter))
      (Variables|Default|SetPhysicsCapsuleRef (Variables|/Script/Engine.Character|GetCapsuleComponent _output_get))
      (Physics|SetSimulatePhysics (Variables|Default|GetPhysicsCapsuleRef) true)
      (Physics|SetEnableGravity (Variables|Default|GetPhysicsCapsuleRef) false)
      (Variables|/Script/Engine.CharacterMovementComponent|SetGravityScale (Variables|/Script/Engine.Character|GetCharacterMovement (Variables|Default|GetOwningCharacterRef)) 0.0)
      (Class|PrimitiveComponent|SetLinearDamping (Variables|Default|GetPhysicsCapsuleRef) (Variables|Toggleable|GetLinearDamping))
      (Class|PrimitiveComponent|SetAngularDamping (Variables|Default|GetPhysicsCapsuleRef) (Variables|Toggleable|GetAngularDamping)))
    (:CastFailed
      (Development|PrintString "Controlled Pawn wasn't a character"))))

(event EventTick
  (params (DeltaSeconds :type Float%20%28single-precision%29)))