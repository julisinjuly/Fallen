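; BP_Angel is an Angel enemy that hurts the player on overlap and can be killed.
; On BeginPlay it passes its behavior tree and the player pawn, as sensing target, to its AI controller.
; While overlapping the first-person character, it applies damage, using a looping timer set by function name.
; Incoming damage is scaled up, updates its health widget, and at zero triggers a particle effect and delayed destruction.
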(event Custom|Damage%20the%20MC
  ;[0.03021 0.03021 0.03021] Damage system
  (if (Variables|Default|GetbIsOverlappingCharacter?)
    (Utilities|Time|SetTimerbyFunctionName 0 "Damage the MC" 0.1 true)
    (Game|Damage|ApplyDamage (Variables|Default|GetCharacterRef) 5.0 0 0)))

(event EventBeginPlay
  ;[0.03854 0.03854 0.03854] Setting up AI controller
  (bind _asai_angels_controller (Utilities|Casting|CastToAI_AngelsController (AI|GetAIController self)))
  (Default|SetUpAIC _asai_angels_controller (Variables|Default|GetBT) (Game|Player|GetPlayerPawn 0)))

(event Collision|EventActorBeginOverlap
  (params (OtherActor :type Actor%20Object%20Reference))
  ;[0.03021 0.03021 0.03021] Damage system
  (bind _asbp_first_person_character (Utilities|Casting|CastToBP_FirstPersonCharacter OtherActor))
  (Variables|Default|SetCharacterRef _asbp_first_person_character)
  (Variables|Default|SetbIsOverlappingCharacter? true)
  (CallFunction|DamagetheMC))

(event Collision|EventActorEndOverlap
  (params (OtherActor :type Actor%20Object%20Reference))
  ;[0.03021 0.03021 0.03021] Damage system
  (Variables|Default|SetbIsOverlappingCharacter? false))

(event Game|Damage|EventAnyDamage
  (params (Damage :type Float%20%28single-precision%29) (DamageType :type Damage%20Type%20Object%20Reference) (InstigatedBy :type Controller%20Object%20Reference) (DamageCauser :type Actor%20Object%20Reference))
  (bind _output_get (Variables|Health|SetCurrentHealth (- (Variables|Health|GetCurrentHealth) (* Damage 1e+02))))
  (bind _aswbp_enemy_health (Utilities|Casting|CastToWBP_EnemyHealth (UserInterface|GetUserWidgetObject (Variables|Default|GetWidget))))
  (bind _output_get_2 (Variables|Default|SetWBPEnemyHealth _aswbp_enemy_health))
  (Default|UpdateHealth _output_get_2 (Math|Integer|Clamp(Integer) _output_get 0 (Variables|Health|GetMaxHealth)))
  (if (<= (Variables|Health|GetCurrentHealth) 0)
    (Effects|SpawnEmitterAttached "/Engine/Tutorial/SubEditors/TutorialAssets/TutorialParticleSystem.TutorialParticleSystem" (Variables|Collision|GetCapsuleComponent) "None")
    (Utilities|FlowControl|Delay 2.0)
    (Actor|DestroyActor)))

(fn ConstructionScript)