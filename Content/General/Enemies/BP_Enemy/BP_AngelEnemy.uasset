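; BP_AngelEnemy is an angel enemy driven by the BT_Angels behavior tree, with a health bar widget.
; Halo throwables overlapping its sphere deal random fractional damage, which AnyDamage scales by 100 before updating health and the widget.
; At zero health it spawns a particle effect and destroys itself after a short delay.
; AngelsAttack sphere-traces forward for the first-person character, then plays a montage and applies damage.
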(event OnComponentBeginOverlap(Sphere)
  (params (OverlappedComponent :type Primitive%20Component%20Object%20Reference) (OtherActor :type Actor%20Object%20Reference) (OtherComp :type Primitive%20Component%20Object%20Reference) (OtherBodyIndex :type Integer) (bFromSweep :type Boolean) (SweepResult :type Hit%20Result%20Structure%20%28by%20ref%29))
  ;[0.06354 0.06354 0.06354] Applying damage
  (Utilities|Casting|CastToBP_HaloThrowable OtherActor)
  (Game|Damage|ApplyDamage self (Math|Random|RandomFloatinRange 0.2 0.35) 0 0)
  (Audio|PlaySoundatLocation 0 "0, 0, 0" "0, 0, 0" 1.0 1.0 0.0 0 0 0 0))

(event Custom|AngelsAttack
  (bind _returnvalue (Transformation|GetActorLocation))
  (bind (_outhit _returnvalue_2) (Collision|SphereTraceForObjects _returnvalue (+ _returnvalue (* (Math|Vector|GetForwardVector (Transformation|GetActorRotation)) 2.5e+02)) 1.2e+02 (Utilities|Array|MakeArray "ObjectTypeQuery3") false 0 "None"))
  (if _returnvalue_2
    (Utilities|Casting|CastToBP_FirstPersonCharacter (.HitActor (Collision|BreakHitResult _outhit)))
    (Animation|Montage|PlayMontage 0 0
      (:then
        (Game|Damage|ApplyDamage (.HitActor (Collision|BreakHitResult _outhit)) 5.0 0 0)))))

(event EventBeginPlay
  ;[0.04271 0.04271 0.04271] Setting Angel Current Health
  (Utilities|FlowControl|Sequence
    (:then_0
      (AI|RunBehaviorTree (AI|GetAIController self) "/Game/General/Enemies/AI_Enemy/BT_Angels.BT_Angels"))
    (:then_1
      (bind _aswbp_enemy_health (Utilities|Casting|CastToWBP_EnemyHealth (UserInterface|GetUserWidgetObject (Variables|Default|GetWidget))))
      (bind _output_get (Variables|Default|SetWBP%20Enemy%20Health _aswbp_enemy_health))
      (Variables|/Game/General/UI/WBP_EnemyHealth.WBP_EnemyHealth_C|SetCurrentHealth _output_get (Variables|Default|GetCurrentHealth))
      (Variables|/Game/General/UI/WBP_EnemyHealth.WBP_EnemyHealth_C|SetMaxHealth (Variables|Default|GetWBP%20Enemy%20Health) (Variables|Default|GetMaxHealth)))))

(event Game|Damage|EventAnyDamage
  (params (Damage :type Float%20%28single-precision%29) (DamageType :type Damage%20Type%20Object%20Reference) (InstigatedBy :type Controller%20Object%20Reference) (DamageCauser :type Actor%20Object%20Reference))
  ;[0.05937 0.05937 0.05937] Updating Health
  (bind _output_get (Variables|Default|SetCurrentHealth (- (Variables|Default|GetCurrentHealth) (* Damage 1e+02))))
  (Default|UpdateHealth (Variables|Default|GetWBP%20Enemy%20Health) (Math|Integer|Clamp(Integer) _output_get 0 (Variables|Default|GetMaxHealth)))
  (if (<= (Variables|Default|GetCurrentHealth) 0)
    (Effects|SpawnEmitterAttached "/Engine/Tutorial/SubEditors/TutorialAssets/TutorialParticleSystem.TutorialParticleSystem" (Variables|Collision|GetCapsuleComponent) "None")
    (Utilities|FlowControl|Delay 2.0)
    (Actor|DestroyActor self)))

(fn ConstructionScript)