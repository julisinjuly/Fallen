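; BP_HaloThrowable is a thrown halo weapon projectile that damages what it hits and can return to the first-person character.
; On BeginPlay, nested loops overwrite its homing target across angel, principality, power and checkpoint actors, without distance checks.
; A per-tick short trace damages and stops the spinning projectile once, while hit events also apply damage.
; ReturnHalo moves it to the character's mesh, reveals the held halo and destroys the projectile.
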(event Custom|ReturnHalo
  ;[0.04271 0.04271 0.04271] Return the Halo
  (Utilities|FlowControl|DoOnce false
    (:Completed
      (bind _returnvalue (Actor|GetActorOfClass "/Game/FirstPerson/Blueprints/BP_FirstPersonCharacter.BP_FirstPersonCharacter_C"))
      (Components|MoveComponentTo (Variables|Default|GetDefaultSceneRoot) (.location (Transformation|GetWorldTransform (Variables|/Script/Engine.Character|GetMesh _returnvalue))) (.rotation (Transformation|GetWorldTransform (Variables|/Script/Engine.Character|GetMesh _returnvalue))) false false 0.2 false)
      (Rendering|SetVisibility (Variables|/Game/FirstPerson/Blueprints/BP_FirstPersonCharacter.BP_FirstPersonCharacter_C|GetHalo1 _returnvalue) true false)
      (Actor|DestroyActor self))))

(event EventBeginPlay
  ;[0.05937 0.05937 0.05937] Auto Aim
  (bind _outactors (Actor|GetAllActorsOfClass "/Game/General/Enemies/Angel_Enemy/Angel/BP_Angel.BP_Angel_C"))
  (for _array_element _outactors
    (Variables|/Script/Engine.ProjectileMovementComponent|SetHomingTargetComponent (Variables|Default|GetProjectileMovement) (Variables|/Script/Engine.Actor|GetRootComponent _array_element))
    (bind _outactors_2 (Actor|GetAllActorsOfClass "/Game/General/Enemies/Principalities/BP_Principalities.BP_Principalities_C"))
    (for _array_element_2 _outactors_2
      (Variables|/Script/Engine.ProjectileMovementComponent|SetHomingTargetComponent (Variables|Default|GetProjectileMovement) (Variables|/Script/Engine.Actor|GetRootComponent _array_element_2))
      (bind _outactors_3 (Actor|GetAllActorsOfClass "/Game/General/Enemies/Powers_Enemies/BP_Powers.BP_Powers_C"))
      (for _array_element_3 _outactors_3
        (Variables|/Script/Engine.ProjectileMovementComponent|SetHomingTargetComponent (Variables|Default|GetProjectileMovement) (Variables|/Script/Engine.Actor|GetRootComponent _array_element_3))
        (bind _outactors_4 (Actor|GetAllActorsOfClass "/Game/General/ChechPoints/BP_Checkpoint.BP_Checkpoint_C"))
        (for _array_element_4 _outactors_4
          (Variables|/Script/Engine.ProjectileMovementComponent|SetHomingTargetComponent (Variables|Default|GetProjectileMovement) (Variables|/Script/Engine.Actor|GetRootComponent _array_element_4)))))))

(event Collision|EventHit
  (params (MyComp :type Primitive%20Component%20Object%20Reference) (Other :type Actor%20Object%20Reference) (OtherComp :type Primitive%20Component%20Object%20Reference) (bSelfMoved :type Boolean) (HitLocation :type Vector :default "0, 0, 0") (HitNormal :type Vector :default "0, 0, 0") (NormalImpulse :type Vector :default "0, 0, 0") (Hit :type Hit%20Result%20Structure%20%28by%20ref%29))
  ;[0.04271 0.04271 0.04271] Throwing a Halo
  (Game|Damage|ApplyDamage (.HitActor (Collision|BreakHitResult Hit)) 0.36 0 0)
  (Utilities|Casting|CastToBP_Checkpoint Other))

(event EventTick
  (params (DeltaSeconds :type Float%20%28single-precision%29))
  (bind _detection_point (Variables|Default|GetDetection%20Point))
  (bind _returnvalue (Transformation|GetWorldLocation _detection_point))
  ;[0.04271 0.04271 0.04271] Throwing a Halo
  (bind (_outhit _returnvalue_2) (Collision|LineTraceByChannel (Transformation|GetWorldLocation (Variables|Default|GetDetection%20Point)) (Math|Vector|MakeVector (+ (.x _returnvalue) 1.0) (.y _returnvalue) (.z _returnvalue)) "TraceTypeQuery1" false (Utilities|Array|MakeArray (Variables|Default|GetSelfRef)) "ForDuration"))
  (if _returnvalue_2
    (Utilities|FlowControl|DoOnce false
      (:Completed
        (Game|Damage|ApplyDamage (.hitactor _outhit) 0.36 0 0)
        (Components|Movement|StopMovementImmediately (Variables|Default|GetProjectileMovement))
        (Variables|/Script/Engine.RotatingMovementComponent|SetRotationRate (Variables|Default|GetRotatingMovement) "0, 0, 0")
        (Variables|/Script/Engine.ProjectileMovementComponent|SetProjectileGravityScale (Variables|Default|GetProjectileMovement) 0.0)
        (Utilities|FlowControl|Delay 2.0)))))

(fn ConstructionScript)