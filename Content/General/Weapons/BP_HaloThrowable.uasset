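; Thrown halo weapon projectile that damages what it strikes, stops, and can return to the player.
; Each tick, a very short visibility trace from DetectionPoint ignores Angel; the first hit applies damage once and halts projectile movement, spin and gravity.
; ReturnHalo runs once, moving the root toward the first-person character's mesh, making Halo visible and destroying the actor.
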(event Custom|ReturnHalo
  ;[0.04271 0.04271 0.04271] Return the Halo
  (Utilities|FlowControl|DoOnce false
    (:Completed
      (bind _returnvalue (Actor|GetActorOfClass "/Game/FirstPerson/Blueprints/BP_FirstPersonCharacter.BP_FirstPersonCharacter_C"))
      (Components|MoveComponentTo (Variables|Default|GetDefaultSceneRoot) (.location (Transformation|GetWorldTransform (Variables|/Script/Engine.Character|GetMesh _returnvalue))) (.rotation (Transformation|GetWorldTransform (Variables|/Script/Engine.Character|GetMesh _returnvalue))) false false 0.4 false)
      (Rendering|SetVisibility (Variables|Default|GetHalo) true false)
      (Actor|DestroyActor self))))

(event EventTick
  (params (DeltaSeconds :type Float%20%28single-precision%29))
  (bind _detection_point (Variables|Default|GetDetection%20Point))
  (bind _returnvalue (Transformation|GetWorldLocation _detection_point))
  ;[0.04271 0.04271 0.04271] Throwing a Halo
  (bind (_outhit _returnvalue_2) (Collision|LineTraceByChannel (Transformation|GetWorldLocation (Variables|Default|GetDetection%20Point)) (Math|Vector|MakeVector (+ (.x _returnvalue) 1.0) (.y _returnvalue) (.z _returnvalue)) "TraceTypeQuery1" false (Utilities|Array|MakeArray (Variables|Default|GetAngel)) "ForDuration"))
  (if _returnvalue_2
    (Utilities|FlowControl|DoOnce false
      (:Completed
        (Game|Damage|ApplyDamage (.hitactor _outhit) 0.36 0 0)
        (Components|Movement|StopMovementImmediately (Variables|Default|GetProjectileMovement))
        (Variables|/Script/Engine.RotatingMovementComponent|SetRotationRate (Variables|Default|GetRotatingMovement) "0, 0, 0")
        (Variables|/Script/Engine.ProjectileMovementComponent|SetProjectileGravityScale (Variables|Default|GetProjectileMovement) 0.0)))))

(fn ConstructionScript)