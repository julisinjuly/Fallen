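; Checkpoint bell actor that activates when hit and loads the victory level once all checkpoints are active at the same time.
; The Hit event tags the hit actor, plays a sound and bell montage, then updates its state and counter.
; A victory check compares the count of "Activated"-tagged checkpoints with all checkpoints in the level.
; Activation is temporary: after a one-minute delay the tag, flag and counter revert.
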(event Custom|CheckingVictory
  ;[0.03438 0.03438 0.03438] Checking Victory
  (bind _outactors (Actor|GetAllActorsOfClass "BP_Checkpoint_C"))
  (bind _outactors_2 (Actor|GetAllActorsOfClasswithTag "BP_Checkpoint_C" "Activated"))
  (if (== (Utilities|Array|Length _outactors_2) (Utilities|Array|Length _outactors))
    (Game|OpenLevel(byName) "LVL_Victory")))

(event Collision|EventHit
  (params (MyComp :type Primitive%20Component%20Object%20Reference) (Other :type Actor%20Object%20Reference) (OtherComp :type Primitive%20Component%20Object%20Reference) (bSelfMoved :type Boolean) (HitLocation :type Vector :default "0, 0, 0") (HitNormal :type Vector :default "0, 0, 0") (NormalImpulse :type Vector :default "0, 0, 0") (Hit :type Hit%20Result%20Structure%20%28by%20ref%29))
  (bind _hitactor (Collision|BreakHitResult Hit))
  (Variables|/Script/Engine.Actor|SetTags _hitactor (Variables|Default|GetTagActivated))
  (Audio|PlaySoundatLocation "/Game/General/SoundDesign/SoundSources/CheckPoints/CheckpointActivated1.CheckpointActivated1" (Transformation|GetActorLocation self) "0, 0, 0" 1.0 1.0 0.0 0 0 0 0)
  (Animation|Montage|PlayMontage (Variables|Default|Getbell) "/Game/environment/models/bell/bell_Anim_bell_bones_bell_anim_Montage.bell_Anim_bell_bones_bell_anim_Montage"
    (:then
      (Utilities|FlowControl|Sequence
        (:then_0
          (Variables|Default|SetbIsActivated? true)
          (Variables|Default|SetCheckPointValue (+ (Variables|Default|GetCheckPointValue) 1))
          (Animation|Montage|PlayMontage 0 0
            (:then
              (Development|PrintString "Checkpoint has been activated!")
              (CallFunction|CheckingVictory)
              (Utilities|FlowControl|Delay 6e+01)
              (Variables|Default|SetbIsActivated? false)
              (Variables|/Script/Engine.Actor|SetTags _hitactor (Variables|Default|GetTagDeactivated))
              (Variables|Default|SetCheckPointValue (- (Variables|Default|GetCheckPointValue) 1))
              (Development|PrintString "CheckPoint has been deactivated!"))))
        (:then_1
          (CallFunction|CheckingVictory))))))

(fn ConstructionScript)